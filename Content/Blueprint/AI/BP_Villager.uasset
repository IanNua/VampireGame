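; BP_Villager is a 2D villager NPC that can be damaged, killed, then fed on to heal the vampire player or turned into a thrall.
; A personality component sets its starting state, and a state switch delegates idle, move, patrol and attack to separate components.
; Outer and inner overlap volumes drive detection, chasing and melee, with a Timeline repeating attacks.
; Thrall conversion spawns BP_Thrall only if the game state's thrall counter allows it.
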(event OnComponentEndOverlap(OuterParameter)
  (params (OverlappedComponent :type Primitive%20Component%20Object%20Reference) (OtherActor :type Actor%20Object%20Reference) (OtherComp :type Primitive%20Component%20Object%20Reference) (OtherBodyIndex :type Integer))
  ;[1 1 1] Max Range
  (if (== OtherActor (Variables|Default|GetAs%20BP%20Vampire%20Character))
    (Variables|Default|SetAIState "NewEnumerator2")
    (CallFunction|SetAIState)
    (else
      (Variables|Default|SetAIState "NewEnumerator0")
      (CallFunction|SetAIState))))

(event OnComponentBeginOverlap(InnerParam)
  (params (OverlappedComponent :type Primitive%20Component%20Object%20Reference) (OtherActor :type Actor%20Object%20Reference) (OtherComp :type Primitive%20Component%20Object%20Reference) (OtherBodyIndex :type Integer) (bFromSweep :type Boolean) (SweepResult :type Hit%20Result%20Structure%20%28by%20ref%29))
  ;[1 1 1] Melee
  (if (== OtherActor (Variables|Default|GetAs%20BP%20Vampire%20Character))
    (Variables|Default|SetAIState "NewEnumerator3")
    (CallFunction|SetAIState)))

(event OnComponentBeginOverlap(OuterParameter)
  (params (OverlappedComponent :type Primitive%20Component%20Object%20Reference) (OtherActor :type Actor%20Object%20Reference) (OtherComp :type Primitive%20Component%20Object%20Reference) (OtherBodyIndex :type Integer) (bFromSweep :type Boolean) (SweepResult :type Hit%20Result%20Structure%20%28by%20ref%29))
  (bind _as_bp_vampire_character (Variables|Default|GetAs%20BP%20Vampire%20Character))
  ;[1 1 1] Max Range
  (if (== OtherActor _as_bp_vampire_character)
    (Class|BIDetection|PlayerDetected(Message) _as_bp_vampire_character 0.2)
    (Variables|Default|SetAIState "NewEnumerator1")
    (CallFunction|SetAIState)))

(event OnComponentEndOverlap(InnerParam)
  (params (OverlappedComponent :type Primitive%20Component%20Object%20Reference) (OtherActor :type Actor%20Object%20Reference) (OtherComp :type Primitive%20Component%20Object%20Reference) (OtherBodyIndex :type Integer))
  ;[1 1 1] Melee
  (if (== OtherActor (Variables|Default|GetAs%20BP%20Vampire%20Character))
    (Variables|Default|SetAIState "NewEnumerator1")
    (CallFunction|SetAIState)
    (else
      (Variables|Default|SetAIState "NewEnumerator2")
      (CallFunction|SetAIState))))

(event Custom|SetAIState
  (bind _aimovestatecomponent (Variables|Default|GetAIMoveStateComponent))
  ;[1 1 1] AI State Machine
  (switch Utilities|FlowControl|Switch|SwitchonE_AIStates (Variables|Default|GetAIState)
    (:NewEnumerator0
      (Default|Idle (Variables|Default|GetAIIdleStateComponent)))
    (:NewEnumerator1
      (Default|MovementType _aimovestatecomponent))
    (:NewEnumerator2
      (Default|MovePatrol (Variables|Default|GetAIPatrolStateComponent)))
    (:NewEnumerator3
      (Default|MovementType _aimovestatecomponent :!label _label)
      (Default|Attack (Variables|Default|GetAIAttackStateComponent))
      (Timeline|Timeline PlayFromStart
        (:Finished
          (goto _label))))))

(event EventBeginPlay
  ;[1 1 1] Event Begin Play
  (bind _asbp_vampire_character (Utilities|Casting|CastToBP_VampireCharacter (Game|GetPlayerCharacter 0)))
  (Variables|Default|SetAs%20BP%20Vampire%20Character _asbp_vampire_character)
  (switch Utilities|FlowControl|Switch|SwitchonE_AIBehviourStates (Variables|/Game/AIPersonalityState.AIPersonalityState_C|GetBehaviour (Variables|Default|GetAIPersonalityState))
    (:NewEnumerator0
      (Variables|Default|SetAIState "NewEnumerator2")
      (CallFunction|SetAIState))
    (:NewEnumerator1
      (Variables|Default|SetAIState "NewEnumerator0")
      (CallFunction|SetAIState))
    (:NewEnumerator2
      (Variables|Default|SetAIState "NewEnumerator0")
      (CallFunction|SetAIState))))

(event Collision|EventActorBeginOverlap
  (params (OtherActor :type Actor%20Object%20Reference)))

(event EventTick
  (params (DeltaSeconds :type Float%20%28single-precision%29)))

(event EventDamageNPC
  (params (DamageAmount :type Float%20%28double-precision%29))
  ;[1 1 1] NPC Take Damage
  (bind _output_get (Variables|Default|SetHealth (- (Variables|Default|GetHealth) DamageAmount)))
  (Development|PrintString (Utilities|String|ToString(Float) _output_get))
  (if (<= _output_get 0.0)
    (Variables|Default|SetHealth 0.0)
    (Variables|/Script/Engine.FloatingPawnMovement|SetMaxSpeed (Variables|Default|GetFloatingPawnMovement) 0.0)
    (Sprite|SetFlipbook (Variables|Default|GetPaperFlipbook) "/Game/Blueprint/ArtPass1/Villager/DeadVillager1.DeadVillager1")))

(event EventFeedNPC
  ;[1 1 1] Be Fed on
  (if (<= (Variables|Default|GetHealth) 0.0)
    (Class|BIHealVampire|HealVampire(Message) (Game|GetPlayerCharacter 0) 0.1)
    (Actor|DestroyActor)))

(event EventTurntoThrall
  ;[1 1 1] Turn To Thrall
  (if (<= (Variables|Default|GetHealth) 0.01)
    (bind _canthrall (Class|BIThrallHandler|ThrallCounter(Message) (Game|GetGameState)))
    (if _canthrall
      (Actor|DestroyActor)
      (Game|SpawnActorfromClass "/Game/Blueprint/AI/BP_Thrall.BP_Thrall_C" (Math|Conversions|ToTransform(Vector) (Transformation|GetActorLocation)) "Undefined" "MultiplyWithRoot" 0 0)
      (else
        (Actor|DestroyActor)))))

(fn ConstructionScript
  (bind _aipatrolstatecomponent (Variables|Default|GetAIPatrolStateComponent))
  ;[1 1 1] Movementlocation
  (Variables|/Game/AIPatrolStateComponent.AIPatrolStateComponent_C|SetStartPoint _aipatrolstatecomponent (Variables|PatrolAI|GetStart%20Point))
  (Variables|/Game/AIPatrolStateComponent.AIPatrolStateComponent_C|SetEndPoint _aipatrolstatecomponent (Variables|PatrolAI|GetEnd%20Point))
  (Default|SetPersonality (Variables|Default|GetAIPersonalityState)))