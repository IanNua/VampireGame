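; BP_Thrall is a Paper2D minion that registers itself in the player vampire's Thrall list on BeginPlay.
; When the player enters its sphere, it runs an AI move toward them, alongside a debug line trace whose result is unused.
; Death notifies the game state, then destroys the actor after a brief delay.
; It also handles axis movement input, and has a directional flipbook handler that is never called.
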(event OnComponentBeginOverlap(Sphere)
  (params (OverlappedComponent :type Primitive%20Component%20Object%20Reference) (OtherActor :type Actor%20Object%20Reference) (OtherComp :type Primitive%20Component%20Object%20Reference) (OtherBodyIndex :type Integer) (bFromSweep :type Boolean) (SweepResult :type Hit%20Result%20Structure%20%28by%20ref%29))
  (bind _self self)
  (bind _as_bp_vampire_character (Variables|Default|GetAs%20BP%20Vampire%20Character))
  (bind _returnvalue (Transformation|GetActorLocation _as_bp_vampire_character))
  (if (== OtherActor _as_bp_vampire_character)
    (Development|PrintString "Hello")
    (Collision|LineTraceByChannel (Transformation|GetActorLocation _self) _returnvalue "TraceTypeQuery1" false 0 "ForOneFrame")
    (AI|AIMoveTo _self _returnvalue _as_bp_vampire_character 5.0 false)))

(event EventBeginPlay
  (bind _asbp_vampire_character (Utilities|Casting|CastToBP_VampireCharacter (Game|GetPlayerCharacter 0)))
  (bind _output_get (Variables|Default|SetAs%20BP%20Vampire%20Character _asbp_vampire_character))
  (Utilities|Array|AddUnique (Variables|/Game/Blueprint/Player/BP_VampireCharacter.BP_VampireCharacter_C|GetThrall _output_get) self))

(event Collision|EventActorBeginOverlap
  (params (OtherActor :type Actor%20Object%20Reference)))

(event EventTick
  (params (DeltaSeconds :type Float%20%28single-precision%29)))

(event EventThrallDeath
  (Development|PrintString "Play death anim")
  (bind _asgs_vampire_game_state (Utilities|Casting|CastToGS_VampireGameState (Game|GetGameState)))
  (Default|RemoveThrallUpdate _asgs_vampire_game_state)
  (Utilities|FlowControl|Delay 0.2)
  (Actor|DestroyActor))

(event Input|AxisEvents|InputAxisMoveUpandDown
  (params (AxisValue :type Float%20%28single-precision%29))
  (Pawn|Input|AddMovementInput "1.000000,0.000000, 0" AxisValue false))

(event Input|AxisEvents|InputAxisMoveRightandLeft
  (params (AxisValue :type Float%20%28single-precision%29))
  (Pawn|Input|AddMovementInput "0.000000,1.000000, 0" AxisValue false))

(fn ConstructionScript)

(fn AnimHandler
  (if (or (!= (Input|AxisValues|GetMoveUpandDown) 0.0) (!= (Input|AxisValues|GetMoveRightandLeft) 0.0))
    (bind _output_get (Variables|Default|SetCurrentDirection (select (> (Input|AxisValues|GetMoveUpandDown) 0.0) "NewEnumerator0" (select (< (Input|AxisValues|GetMoveUpandDown) 0.0) "NewEnumerator1" (select (> (Input|AxisValues|GetMoveRightandLeft) 0.0) "NewEnumerator3" "NewEnumerator2")))))
    (Sprite|SetFlipbook (Variables|Default|GetPaperFlipbook) (Utilities|Select :Index _output_get :NewEnumerator0 0 :NewEnumerator1 0 :NewEnumerator2 0 :NewEnumerator3 0))
    (else
      (Sprite|SetFlipbook (Variables|Default|GetPaperFlipbook) (Utilities|Select :Index _output_get :NewEnumerator0 0 :NewEnumerator1 0 :NewEnumerator2 0 :NewEnumerator3 0)))))