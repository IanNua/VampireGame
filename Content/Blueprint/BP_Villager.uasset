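; BP_Villager is a Paper2D villager NPC that the player vampire can damage and feed on.
; DamageNPC lowers Health; at zero it stops floating-pawn movement and shows a dead flipbook.
; FeedNPC works only on a dead villager, sending a heal message to the player before destroying it.
; Sphere overlap with BP_VampireCharacter triggers AIMoveTo toward the vampire, after a debug-drawn line trace whose result is ignored.
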(event OnComponentBeginOverlap(Sphere)
  (params (OverlappedComponent :type Primitive%20Component%20Object%20Reference) (OtherActor :type Actor%20Object%20Reference) (OtherComp :type Primitive%20Component%20Object%20Reference) (OtherBodyIndex :type Integer) (bFromSweep :type Boolean) (SweepResult :type Hit%20Result%20Structure%20%28by%20ref%29))
  (bind _self self)
  (bind _asbp_vampire_character (Utilities|Casting|CastToBP_VampireCharacter OtherActor))
  (Development|PrintString "Hello")
  (Collision|LineTraceByChannel (Transformation|GetActorLocation _self) (Transformation|GetActorLocation _asbp_vampire_character) "TraceTypeQuery1" false 0 "ForOneFrame")
  (AI|AIMoveTo _self (Transformation|GetActorLocation _asbp_vampire_character) _asbp_vampire_character 5.0 false))

(event EventBeginPlay)

(event Collision|EventActorBeginOverlap
  (params (OtherActor :type Actor%20Object%20Reference)))

(event EventTick
  (params (DeltaSeconds :type Float%20%28single-precision%29)))

(event EventDamageNPC
  (params (DamageAmount :type Float%20%28double-precision%29))
  ;[1 1 1] NPC Take Damage
  (bind _output_get (Variables|Default|SetHealth (- (Variables|Default|GetHealth) DamageAmount)))
  (Development|PrintString (Utilities|String|ToString(Float) _output_get))
  (if (<= _output_get 0.0)
    (Variables|Default|SetHealth 0.0)
    (Variables|/Script/Engine.FloatingPawnMovement|SetMaxSpeed (Variables|Default|GetFloatingPawnMovement) 0.0)
    (Sprite|SetFlipbook (Variables|Default|GetPaperFlipbook) "/Game/Blueprint/ArtPass1/Villager/DeadVillager1.DeadVillager1")))

(event EventFeedNPC
  (if (<= (Variables|Default|GetHealth) 0.0)
    (Class|BIHealVampire|HealVampire(Message) (Game|GetPlayerCharacter 0) 0.1)
    (Actor|DestroyActor)))

(fn ConstructionScript)