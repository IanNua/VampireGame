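; BP_Thrall is a flipbook-animated thrall pawn that registers itself with the player's BP_VampireCharacter on BeginPlay.
; When the vampire enters its sphere, it prints a debug message, runs an unused line trace and issues AIMoveTo toward the vampire.
; It also takes world-axis movement input directly.
; AnimHandler picks directional moving or idle flipbooks from that input, but its call is unconnected, so it never runs.
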(event OnComponentBeginOverlap(Sphere)
  (params (OverlappedComponent :type Primitive%20Component%20Object%20Reference) (OtherActor :type Actor%20Object%20Reference) (OtherComp :type Primitive%20Component%20Object%20Reference) (OtherBodyIndex :type Integer) (bFromSweep :type Boolean) (SweepResult :type Hit%20Result%20Structure%20%28by%20ref%29))
  (bind _self self)
  (bind _asbp_vampire_character (Utilities|Casting|CastToBP_VampireCharacter OtherActor))
  (Development|PrintString "Hello")
  (Collision|LineTraceByChannel (Transformation|GetActorLocation _self) (Transformation|GetActorLocation _asbp_vampire_character) "TraceTypeQuery1" false 0 "ForOneFrame")
  (AI|AIMoveTo _self (Transformation|GetActorLocation _asbp_vampire_character) _asbp_vampire_character 5.0 false))

(event EventBeginPlay
  (bind _asbp_vampire_character (Utilities|Casting|CastToBP_VampireCharacter (Game|GetPlayerCharacter 0)))
  (Variables|/Game/Blueprint/Player/BP_VampireCharacter.BP_VampireCharacter_C|SetThrall _asbp_vampire_character self))

(event Collision|EventActorBeginOverlap
  (params (OtherActor :type Actor%20Object%20Reference)))

(event EventTick
  (params (DeltaSeconds :type Float%20%28single-precision%29)))

(event Input|AxisEvents|InputAxisMoveUpandDown
  (params (AxisValue :type Float%20%28single-precision%29))
  (Pawn|Input|AddMovementInput "1.000000,0.000000, 0" AxisValue false))

(event Input|AxisEvents|InputAxisMoveRightandLeft
  (params (AxisValue :type Float%20%28single-precision%29))
  (Pawn|Input|AddMovementInput "0.000000,1.000000, 0" AxisValue false))

(fn ConstructionScript)

(fn AnimHandler
  (if (or (!= (Input|AxisValues|GetMoveUpandDown) 0.0) (!= (Input|AxisValues|GetMoveRightandLeft) 0.0))
    (bind _output_get (Variables|Default|SetCurrentDirection (select (> (Input|AxisValues|GetMoveUpandDown) 0.0) "NewEnumerator0" (select (< (Input|AxisValues|GetMoveUpandDown) 0.0) "NewEnumerator1" (select (> (Input|AxisValues|GetMoveRightandLeft) 0.0) "NewEnumerator3" "NewEnumerator2")))))
    (Sprite|SetFlipbook (Variables|Default|GetPaperFlipbook) (Utilities|Select :Index _output_get :NewEnumerator0 0 :NewEnumerator1 0 :NewEnumerator2 0 :NewEnumerator3 0))
    (else
      (Sprite|SetFlipbook (Variables|Default|GetPaperFlipbook) (Utilities|Select :Index _output_get :NewEnumerator0 0 :NewEnumerator1 0 :NewEnumerator2 0 :NewEnumerator3 0)))))