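; BP_VampireCharacter is a player-controlled vampire character with movement, sprint and bat-mode inputs.
; Two axis inputs move it along fixed world X and Y, and Sprint doubles CharacterMovement's max walk speed while held.
; BatMode uses a FlipFlop to toggle the vampire state enum, starting from its BeginPlay default, without changing mesh or movement.
; Attack, Feed and Bite are placeholders that only print debug strings.
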(event EventBeginPlay
  (Variables|Default|SetCurrentVampireState "NewEnumerator0"))

(event Collision|EventActorBeginOverlap
  (params (OtherActor :type Actor%20Object%20Reference)))

(event EventTick
  (params (DeltaSeconds :type Float%20%28single-precision%29))
  ;[1 0.05251 0] Debug Only
)

(event Input|ActionEvents|InputActionAttack
  (params (Key :type Key%20Structure :default "None"))
  (:Pressed
    (Development|PrintString "Attack")))

(event Input|ActionEvents|InputActionFeed
  (params (Key :type Key%20Structure :default "None"))
  (:Pressed
    (Development|PrintString "Feed")))

(event Input|ActionEvents|InputActionBatMode
  (params (Key :type Key%20Structure :default "None"))
  ;[1 1 1] BatMode Turns to Bat or Vampire
  (:Pressed
    (Utilities|FlowControl|FlipFlop
      (:A
        (bind _output_get (Variables|Default|SetCurrentVampireState "NewEnumerator1"))
        (Development|PrintString (Utilities|String|EnumtoString _output_get)))
      (:B
        (bind _output_get_2 (Variables|Default|SetCurrentVampireState "NewEnumerator0"))
        (Development|PrintString (Utilities|String|EnumtoString _output_get_2))))))

(event Input|ActionEvents|InputActionBite
  (params (Key :type Key%20Structure :default "None"))
  (:Pressed
    (Development|PrintString "BiteNOM")))

(event Input|ActionEvents|InputActionSprint
  (params (Key :type Key%20Structure :default "None"))
  (bind _charactermovement (Variables|Character|GetCharacterMovement))
  ;[1 1 1] Sprint Doubles Player Speed
  (:Pressed
    (Development|PrintString "SPRINT")
    (Variables|/Script/Engine.CharacterMovementComponent|SetMaxWalkSpeed _charactermovement 1.2e+03))
  (:Released
    (Variables|/Script/Engine.CharacterMovementComponent|SetMaxWalkSpeed _charactermovement 6e+02)))

(event Input|AxisEvents|InputAxisMoveRightandLeft
  (params (AxisValue :type Float%20%28single-precision%29))
  (Pawn|Input|AddMovementInput "0.000000,1.000000, 0" AxisValue false))

(event Input|AxisEvents|InputAxisMoveUpandDown
  (params (AxisValue :type Float%20%28single-precision%29))
  (Pawn|Input|AddMovementInput "1.000000,0.000000, 0" AxisValue false))

(fn ConstructionScript)