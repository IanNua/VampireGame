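; Game state for a vampire game that keeps a running count of thralls and limits it against MaxThralls.
; ThrallCounter increments the count first, then rolls it back and returns false if it reaches MaxThralls, so the accepted count stays below that value.
; RemoveThrallUpdate decrements the count, and the event graph holds no active logic.
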(event EventBeginPlay)

(event EventTick
  (params (DeltaSeconds :type Float%20%28single-precision%29)))

(fn ConstructionScript)

(fn RemoveThrallUpdate
  (Utilities|RemoveThrall))

(fn ThrallCounter
  (bind _output_get (Utilities|AddThrall))
  (if (>= _output_get (LocalVariables|GetMaxThralls))
    (Utilities|RemoveThrall)
    (return false)
    (else
      (return true))))