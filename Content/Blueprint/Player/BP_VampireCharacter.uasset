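; Player vampire character using Paper2D flipbooks, with bat transformation, sprint, attack, feed and bite-to-thrall abilities.
; Input sets action and state enums, which AnimHandeller combines with facing direction to pick flipbooks.
; Attack, feed and bite send messages to the actor hit by a short directional line trace.
; Health and stamina live in components; StaminaChecker only resets the action without blocking it, and Death is never called here.
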(event OnFinishedPlaying(PaperFlipbook))

(event EventBeginPlay
  (Variables|Default|SetCurrentVampireState "NewEnumerator0")
  (bind _returnvalue (UserInterface|CreateWidget "/Game/UMG/UMG_HUD.UMG_HUD_C" 0 self))
  (UserInterface|Viewport|AddtoViewport _returnvalue 0))

(event Collision|EventActorBeginOverlap
  (params (OtherActor :type Actor%20Object%20Reference)))

(event EventPlayerDetected
  (params (Detection :type Float%20%28double-precision%29))
  (bind _output_get (Variables|Default|SetDetection (+ Detection (Variables|Default|GetDetection))))
  (if (> (Math|Float|Clamp(Float) _output_get) 0.5)
    (Development|PrintString "detected")
    (else
      (Development|PrintString "NOT detected"))))

(event EventTick
  (params (DeltaSeconds :type Float%20%28single-precision%29))
  ;[1 0.05251 0] Debug Only
)

(event EventHealVampire
  (params (HealAmount :type Float%20%28double-precision%29))
  (Default|Heal (Variables|Default|GetDamageComponent) HealAmount))

(event Input|ActionEvents|InputActionFeed
  (params (Key :type Key%20Structure))
  ;[1 1 1] Feed System
  (:Pressed
    (Development|PrintString "Feed")
    (Default|StaminaGain (Variables|Default|GetStaminaComponent) 1.0)
    (Variables|Default|SetCurrentAction "NewEnumerator2")
    (bind _hitactor (CallFunction|ObjectCheckingFunction))
    (CallFunction|AnimHandeller)
    (Class|BIFeedNPC|FeedNPC(Message) _hitactor))
  (:Released
    (Variables|Default|SetCurrentAction "NewEnumerator0")))

(event Input|ActionEvents|InputActionBatMode
  (params (Key :type Key%20Structure))
  (bind _charactermovement (Variables|Character|GetCharacterMovement))
  (:Pressed
    ;[1 1 1] BatMode Turns to Bat or Vampire
    (CallFunction|StaminaChecker)
    (Utilities|FlowControl|FlipFlop
      (:A
        (Default|StaminaLose (Variables|Default|GetStaminaComponent) 0.2)
        (bind _output_get (Variables|Default|SetCurrentVampireState "NewEnumerator1"))
        (Development|PrintString (Utilities|String|EnumtoString _output_get))
        (Variables|/Script/Engine.CharacterMovementComponent|SetMaxWalkSpeed _charactermovement 9e+02))
      (:B
        (bind _output_get_2 (Variables|Default|SetCurrentVampireState "NewEnumerator0"))
        (Development|PrintString (Utilities|String|EnumtoString _output_get_2))
        (Variables|/Script/Engine.CharacterMovementComponent|SetMaxWalkSpeed _charactermovement 6e+02)))))

(event Input|ActionEvents|InputActionBite
  (params (Key :type Key%20Structure))
  ;[1 1 1] Bite System Turn to Thrall
  (:Pressed
    (Development|PrintString "BiteNOM")
    (Default|StaminaGain (Variables|Default|GetStaminaComponent) 1.0)
    (Variables|Default|SetCurrentAction "NewEnumerator3")
    (bind _hitactor (CallFunction|ObjectCheckingFunction))
    (CallFunction|AnimHandeller)
    (CallFunction|BiteAction _hitactor))
  (:Released
    (Variables|Default|SetCurrentAction "NewEnumerator0")))

(event Input|ActionEvents|InputActionSprint
  (params (Key :type Key%20Structure))
  (bind _charactermovement (Variables|Character|GetCharacterMovement))
  (:Pressed
    (CallFunction|StaminaChecker)
    ;[1 1 1] Sprint Doubles Player Speed
    (Default|StaminaLose (Variables|Default|GetStaminaComponent) 0.1)
    (Development|PrintString "SPRINT ON")
    (Variables|/Script/Engine.CharacterMovementComponent|SetMaxWalkSpeed _charactermovement 6e+02)
    (Variables|Default|SetCurrentAction "NewEnumerator1"))
  (:Released
    (Development|PrintString "SPRINT OFF")
    (Variables|/Script/Engine.CharacterMovementComponent|SetMaxWalkSpeed _charactermovement 3e+02)
    (Variables|Default|SetCurrentAction "NewEnumerator0")))

(event Input|ActionEvents|InputActionAttack
  (params (Key :type Key%20Structure))
  (:Pressed
    ;[1 1 1] Attack System
    (CallFunction|StaminaChecker)
    (Default|StaminaLose (Variables|Default|GetStaminaComponent) 0.1)
    (Development|PrintString "Attack")
    (Variables|Default|SetCurrentAction "NewEnumerator4")
    (bind _hitactor (CallFunction|ObjectCheckingFunction))
    (Development|PrintString (Utilities|GetDisplayName _hitactor))
    (CallFunction|AnimHandeller)
    (Class|BIDamageNPC|DamageNPC(Message) _hitactor (Variables|Default|GetAttackAmount)))
  (:Released
    (Variables|Default|SetCurrentAction "NewEnumerator0")))

(event Input|AxisEvents|InputAxisMoveRightandLeft
  (params (AxisValue :type Float%20%28single-precision%29))
  (Pawn|Input|AddMovementInput "0.000000,1.000000, 0" AxisValue false)
  (CallFunction|AnimHandeller))

(event Input|AxisEvents|InputAxisMoveUpandDown
  (params (AxisValue :type Float%20%28single-precision%29))
  (Pawn|Input|AddMovementInput "1.000000,0.000000, 0" AxisValue false)
  (CallFunction|AnimHandeller))

(event Input|KeyboardEvents|Q
  (params (Key :type Key%20Structure))
  (:Pressed
    (Default|DamageSingle (Variables|Default|GetDamageComponent) 0.1)))

(fn ConstructionScript
  (bind _staminacomponent (Variables|Default|GetStaminaComponent))
  (bind _damagecomponent (Variables|Default|GetDamageComponent))
  (bind _output_get (Variables|/Game/HealthComponent.HealthComponent_C|SetMaxHealth _damagecomponent 1.0))
  (Variables|/Game/HealthComponent.HealthComponent_C|SetCurrentHealth _damagecomponent _output_get)
  (bind _output_get_2 (Variables|/Game/StaminaComponent.StaminaComponent_C|SetMaxStamina _staminacomponent 1.0))
  (Variables|/Game/StaminaComponent.StaminaComponent_C|SetCurrentStamina _staminacomponent _output_get_2))

(fn AnimHandeller
  (if (or (!= (Input|AxisValues|GetMoveUpandDown) 0.0) (!= (Input|AxisValues|GetMoveRightandLeft) 0.0))
    (Variables|Default|SetCurrentDirection (select (> (Input|AxisValues|GetMoveUpandDown) 0.0) "NewEnumerator0" (select (< (Input|AxisValues|GetMoveUpandDown) 0.0) "NewEnumerator1" (select (> (Input|AxisValues|GetMoveRightandLeft) 0.0) "NewEnumerator3" "NewEnumerator2"))))
    (switch Utilities|FlowControl|Switch|Switchone_VampireAction (Variables|Default|GetCurrentAction)
      (:NewEnumerator0
        (CallFunction|WalkingAnimation))
      (:NewEnumerator1
        (CallFunction|SprintAnimation))
      (:NewEnumerator2
        (CallFunction|BiteAnimation :!label _label))
      (:NewEnumerator3
        (goto _label))
      (:NewEnumerator4
        (CallFunction|AttackAnimation))
      (:NewEnumerator6
        (CallFunction|ThrallHandeller)))
    (else
      (switch Utilities|FlowControl|Switch|Switchone_VampireAction (Variables|Default|GetCurrentAction)
        (:NewEnumerator0
          (CallFunction|IdleAnimation))
        (:NewEnumerator2
          (CallFunction|BiteAnimation :!label _label_2))
        (:NewEnumerator3
          (goto _label_2))
        (:NewEnumerator4
          (CallFunction|AttackAnimation))
        (:NewEnumerator6
          (CallFunction|ThrallHandeller))))))

(fn IdleAnimation
  (bind _paperflipbook (Variables|Default|GetPaperFlipbook))
  (switch Utilities|FlowControl|Switch|SwitchonE_VampireState (Variables|Default|GetCurrentVampireState)
    (:NewEnumerator0
      (Sprite|SetFlipbook _paperflipbook (Utilities|Select :Index (Variables|Default|GetCurrentDirection) :NewEnumerator0 "/Game/Blueprint/ArtPass1/Vamp/UpIdleVamp.UpIdleVamp" :NewEnumerator1 "/Game/Blueprint/ArtPass1/Vamp/DownIdleVamp.DownIdleVamp" :NewEnumerator2 "/Game/Blueprint/ArtPass1/Vamp/RightIdleVamp.RightIdleVamp" :NewEnumerator3 "/Game/Blueprint/ArtPass1/Vamp/LeftIdleVamp.LeftIdleVamp")))
    (:NewEnumerator1
      ;[1 1 1] Idle Anim for Bat
      (Sprite|SetFlipbook _paperflipbook (Utilities|Select :Index (Variables|Default|GetCurrentDirection) :NewEnumerator0 "/Game/Blueprint/ArtPass1/Vamp/UpIdleBat.UpIdleBat" :NewEnumerator1 "/Game/Blueprint/ArtPass1/Vamp/DownIdleBat.DownIdleBat" :NewEnumerator2 "/Game/Blueprint/ArtPass1/Vamp/UpIdleBat.UpIdleBat" :NewEnumerator3 "/Game/Blueprint/ArtPass1/Vamp/DownWalkBat.DownWalkBat")))))

(fn WalkingAnimation
  (bind _paperflipbook (Variables|Default|GetPaperFlipbook))
  (switch Utilities|FlowControl|Switch|SwitchonE_VampireState (Variables|Default|GetCurrentVampireState)
    (:NewEnumerator0
      ;[1 1 1] Walking Vampire
      (Sprite|SetFlipbook _paperflipbook (Utilities|Select :Index (Variables|Default|GetCurrentDirection) :NewEnumerator0 "/Game/Blueprint/ArtPass1/Vamp/UpWalkVamp.UpWalkVamp" :NewEnumerator1 "/Game/Blueprint/ArtPass1/Vamp/DownWalkVamp.DownWalkVamp" :NewEnumerator2 "/Game/Blueprint/ArtPass1/Vamp/RightWalkVamp.RightWalkVamp" :NewEnumerator3 "/Game/Blueprint/ArtPass1/Vamp/LeftWalkVamp.LeftWalkVamp")))
    (:NewEnumerator1
      ;[1 1 1] Walking Bat
      (Sprite|SetFlipbook _paperflipbook (Utilities|Select :Index (Variables|Default|GetCurrentDirection) :NewEnumerator0 "/Game/Blueprint/ArtPass1/Vamp/UpWalkBat.UpWalkBat" :NewEnumerator1 "/Game/Blueprint/ArtPass1/Vamp/DownWalkBat.DownWalkBat" :NewEnumerator2 "/Game/Blueprint/ArtPass1/Vamp/UpWalkBat.UpWalkBat" :NewEnumerator3 "/Game/Blueprint/ArtPass1/Vamp/DownWalkBat.DownWalkBat")))))

(fn SprintAnimation
  (bind _paperflipbook (Variables|Default|GetPaperFlipbook))
  (switch Utilities|FlowControl|Switch|SwitchonE_VampireState (Variables|Default|GetCurrentVampireState)
    (:NewEnumerator0
      ;[1 1 1] Sprint Vampire
      (Sprite|SetFlipbook _paperflipbook (Utilities|Select :Index (Variables|Default|GetCurrentDirection) :NewEnumerator0 "/Game/Blueprint/ArtPass1/Vamp/UpWalkVamp.UpWalkVamp" :NewEnumerator1 "/Game/Blueprint/ArtPass1/Vamp/DownWalkVamp.DownWalkVamp" :NewEnumerator2 "/Game/Blueprint/ArtPass1/Vamp/RightWalkVamp.RightWalkVamp" :NewEnumerator3 "/Game/Blueprint/ArtPass1/Vamp/LeftWalkVamp.LeftWalkVamp"))
      (Development|PrintString "Sprinting"))
    (:NewEnumerator1
      ;[1 1 1] Sprint Bat
      (Sprite|SetFlipbook _paperflipbook (Utilities|Select :Index (Variables|Default|GetCurrentDirection) :NewEnumerator0 "/Game/Blueprint/ArtPass1/Vamp/UpWalkBat.UpWalkBat" :NewEnumerator1 "/Game/Blueprint/ArtPass1/Vamp/DownWalkBat.DownWalkBat" :NewEnumerator2 "/Game/Blueprint/ArtPass1/Vamp/UpWalkBat.UpWalkBat" :NewEnumerator3 "/Game/Blueprint/ArtPass1/Vamp/DownWalkBat.DownWalkBat"))
      (Development|PrintString "Sprinting"))))

(fn AttackAnimation
  (bind _paperflipbook (Variables|Default|GetPaperFlipbook))
  (switch Utilities|FlowControl|Switch|SwitchonE_VampireState (Variables|Default|GetCurrentVampireState)
    (:NewEnumerator0
      ;[1 1 1] Sprint Vampire
      (Sprite|SetFlipbook _paperflipbook (Utilities|Select :Index (Variables|Default|GetCurrentDirection) :NewEnumerator0 "/Game/Blueprint/ArtPass1/Vamp/UpAttackVamp.UpAttackVamp" :NewEnumerator1 "/Game/Blueprint/ArtPass1/Vamp/DownAttackVamp.DownAttackVamp" :NewEnumerator2 "/Game/Blueprint/ArtPass1/Vamp/RightAttackVamp.RightAttackVamp" :NewEnumerator3 "/Game/Blueprint/ArtPass1/Vamp/LeftAttackVamp.LeftAttackVamp")))
    (:NewEnumerator1
      ;[1 1 1] Sprint Bat
      (Sprite|SetFlipbook _paperflipbook (Utilities|Select :Index (Variables|Default|GetCurrentDirection) :NewEnumerator0 "/Game/Blueprint/ArtPass1/Vamp/UpWalkBat.UpWalkBat" :NewEnumerator1 "/Game/Blueprint/ArtPass1/Vamp/DownWalkBat.DownWalkBat" :NewEnumerator2 "/Game/Blueprint/ArtPass1/Vamp/UpWalkBat.UpWalkBat" :NewEnumerator3 "/Game/Blueprint/ArtPass1/Vamp/DownWalkBat.DownWalkBat"))
      (Development|PrintString "Attacking"))))

(fn ObjectCheckingFunction
  (bind _self self)
  (bind _returnvalue (Transformation|GetActorLocation _self))
  (switch Utilities|FlowControl|Switch|SwitchonE_VampireDirection (Variables|Default|GetCurrentDirection)
    (:NewEnumerator0
      (bind _outhit (Collision|LineTraceByChannel _returnvalue (+ _returnvalue "50.000000,0,0") "TraceTypeQuery1" false 0 "Persistent"))
      (return (.HitActor (Collision|BreakHitResult _outhit))))
    (:NewEnumerator1
      (bind _outhit_2 (Collision|LineTraceByChannel _returnvalue (- _returnvalue "50.000000,0,0") "TraceTypeQuery1" false 0 "Persistent"))
      (return (.HitActor (Collision|BreakHitResult _outhit_2))))
    (:NewEnumerator2
      (bind _outhit_3 (Collision|LineTraceByChannel _returnvalue (- _returnvalue "0,50.000000,0") "TraceTypeQuery1" false 0 "Persistent" true "(R=1.000000,G=0.756863,B=0.000000,A=1.000000)"))
      (return (.HitActor (Collision|BreakHitResult _outhit_3))))
    (:NewEnumerator3
      (bind _outhit_4 (Collision|LineTraceByChannel _returnvalue (+ _returnvalue "0,50.000000,0") "TraceTypeQuery1" false 0 "Persistent" true "(R=1.000000,G=0.756863,B=0.000000,A=1.000000)"))
      (return (.HitActor (Collision|BreakHitResult _outhit_4))))))

(fn BiteAnimation
  (bind _paperflipbook (Variables|Default|GetPaperFlipbook))
  (switch Utilities|FlowControl|Switch|SwitchonE_VampireState (Variables|Default|GetCurrentVampireState)
    (:NewEnumerator0
      ;[1 1 1] Sprint Vampire
      (Sprite|SetFlipbook _paperflipbook (Utilities|Select :Index (Variables|Default|GetCurrentDirection) :NewEnumerator0 "/Game/Blueprint/ArtPass1/Vamp/UpBiteVamp.UpBiteVamp" :NewEnumerator1 "/Game/Blueprint/ArtPass1/Vamp/DownBiteVamp.DownBiteVamp" :NewEnumerator2 "/Game/Blueprint/ArtPass1/Vamp/RightBiteVamp.RightBiteVamp" :NewEnumerator3 "/Game/Blueprint/ArtPass1/Vamp/LeftBiteVamp.LeftBiteVamp")))
    (:NewEnumerator1
      ;[1 1 1] Sprint Bat
      (Sprite|SetFlipbook _paperflipbook (Utilities|Select :Index (Variables|Default|GetCurrentDirection) :NewEnumerator0 "/Game/Blueprint/ArtPass1/Vamp/UpWalkBat.UpWalkBat" :NewEnumerator1 "/Game/Blueprint/ArtPass1/Vamp/DownWalkBat.DownWalkBat" :NewEnumerator2 "/Game/Blueprint/ArtPass1/Vamp/UpWalkBat.UpWalkBat" :NewEnumerator3 "/Game/Blueprint/ArtPass1/Vamp/DownWalkBat.DownWalkBat")))))

(fn Death
  (if (<= (Variables|/Game/HealthComponent.HealthComponent_C|GetCurrentHealth (Variables|Default|GetDamageComponent)) 0.0)
    (Sprite|SetFlipbook (Variables|Default|GetPaperFlipbook) (Utilities|Select :Index (Variables|Default|GetCurrentDirection) :NewEnumerator0 "/Game/Blueprint/ArtPass1/Vamp/RightDeadVamp.RightDeadVamp" :NewEnumerator1 "/Game/Blueprint/ArtPass1/Vamp/LeftDeadVamp.LeftDeadVamp" :NewEnumerator2 "/Game/Blueprint/ArtPass1/Vamp/RightDeadVamp.RightDeadVamp" :NewEnumerator3 "/Game/Blueprint/ArtPass1/Vamp/LeftDeadVamp.LeftDeadVamp"))
    (Variables|/Script/Engine.CharacterMovementComponent|SetMaxWalkSpeed (Variables|Character|GetCharacterMovement) 0.0)
    (bind _returnvalue (UserInterface|CreateWidget "/Game/UMG/UMG_Death.UMG_Death_C"))
    (UserInterface|Viewport|AddtoViewport _returnvalue 0)))

(fn BiteAction
  (params (HitActor :type Actor%20Object%20Reference))
  (Class|BITurntoThrall|TurntoThrall(Message) HitActor))

(fn ThrallHandeller
  (Variables|Default|SetCurrentVampireState "NewEnumerator2")
  ;[1 1 1] 100% this
  (Sprite|SetFlipbook (Variables|Default|GetPaperFlipbook) (Utilities|Select :Index (Variables|Default|GetCurrentDirection) :NewEnumerator0 "/Game/Blueprint/ArtPass1/Vamp/ThrallVamp.ThrallVamp" :NewEnumerator1 "/Game/Blueprint/ArtPass1/Vamp/ThrallVamp.ThrallVamp" :NewEnumerator2 "/Game/Blueprint/ArtPass1/Vamp/ThrallVamp.ThrallVamp" :NewEnumerator3 "/Game/Blueprint/ArtPass1/Vamp/ThrallVamp.ThrallVamp")))

(fn StaminaChecker
  (if (> (Variables|/Game/StaminaComponent.StaminaComponent_C|GetCurrentStamina (Variables|Default|GetStaminaComponent)) 0.0)
    (return)
    (else
      (Variables|Default|SetCurrentAction "NewEnumerator0"))))