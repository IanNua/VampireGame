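; BP_WaterVolume is a water volume that blocks or admits the player's vampire depending on its current state.
; It caches the player's BP_VampireCharacter on BeginPlay and compares it against actors entering the Box.
; On that overlap, Cube collision turns on for the first CurrentVampireState value and off for any other.
; The state is checked only when overlap begins, with no end-overlap or per-tick update.
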(event OnComponentBeginOverlap(Box)
  (params (OverlappedComponent :type Primitive%20Component%20Object%20Reference) (OtherActor :type Actor%20Object%20Reference) (OtherComp :type Primitive%20Component%20Object%20Reference) (OtherBodyIndex :type Integer) (bFromSweep :type Boolean) (SweepResult :type Hit%20Result%20Structure%20%28by%20ref%29))
  (bind _as_bp_vampire_character (Variables|Default|GetAs%20BP%20Vampire%20Character))
  (bind _cube (Variables|Default|GetCube))
  (if (== OtherActor _as_bp_vampire_character)
    (if (Utilities|Enum|Equal(Enum) (Variables|/Game/Blueprint/Player/BP_VampireCharacter.BP_VampireCharacter_C|GetCurrentVampireState _as_bp_vampire_character) "NewEnumerator0")
      (Collision|SetCollisionEnabled _cube "QueryAndPhysics")
      (else
        (Collision|SetCollisionEnabled _cube "NoCollision")))))

(event EventBeginPlay
  (bind _asbp_vampire_character (Utilities|Casting|CastToBP_VampireCharacter (Game|GetPlayerCharacter 0)))
  (Variables|Default|SetAs%20BP%20Vampire%20Character _asbp_vampire_character))

(event Collision|EventActorBeginOverlap
  (params (OtherActor :type Actor%20Object%20Reference)))

(event EventTick
  (params (DeltaSeconds :type Float%20%28single-precision%29)))

(fn ConstructionScript)